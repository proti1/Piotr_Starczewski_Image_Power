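; Minion AI character that can be told to search for a chosen type of object.
; On BeginPlay it has its AI controller run BT_Minion and use BB_Minion, caching the Blackboard component.
; StartSearchItem stores the requested object enum, writes it to the SearchedObject key and sets bShouldSearch, leaving the search itself to the Behavior Tree.
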(event Custom|StartSearchItem
  (params (ObjectToSearch :type EObjectList%20Enum :default "OL_Nothing"))
  (bind _blackboardref (Variables|Default|GetBlackboardRef))
  ;[1 1 1] Po zakończeniu interfejsu zacznij szukać
  (Variables|Default|SetSearchedObject ObjectToSearch)
  (AI|Components|Blackboard|SetValueasEnum _blackboardref (Utilities|Name|MakeLiteralName "SearchedObject") ObjectToSearch)
  (AI|Components|Blackboard|SetValueasBool _blackboardref (Utilities|Name|MakeLiteralName "bShouldSearch") true))

(event EventBeginPlay
  (bind _self self)
  (bind _returnvalue (AI|GetAIController _self))
  ;[1 1 1] Ustaw Behavior Tree i Blackboard
  (AI|RunBehaviorTree _returnvalue "/Game/Characters/Minion/BT_Minion.BT_Minion")
  (bind _blackboardcomponent (Class|AIController|UseBlackboard _returnvalue "/Game/Characters/Minion/BB_Minion.BB_Minion"))
  (Variables|Default|SetBlackboardRef _blackboardcomponent))

(event Collision|EventActorBeginOverlap
  (params (OtherActor :type Actor%20Object%20Reference)))

(event EventTick
  (params (DeltaSeconds :type Float%20%28single-precision%29)))

(fn ConstructionScript)